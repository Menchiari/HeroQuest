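; BP_Board is a board actor that randomizes the look of its static mesh.
; On BeginPlay it applies a random entry from the Meshes array to material slot 0.
; Seven debug keys, on release, re-roll that slot from themed arrays: Nature, Goblin, Mess, Sewers, Wood, Persian and a default set.
; Despite their Mesh names, these arrays supply materials, so the mesh itself never changes.
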(event EventBeginPlay
  (Rendering|Material|SetMaterial (Variables|Debug|GetStaticMeshComponent) 0 (.OutItem (Utilities|Array|Random (Variables|Default|GetMeshes)))))

(event Input|KeyboardEvents|DebugKey1
  (params (Key :type Key%20Structure :default "None") (ActionValue :type Input%20Action%20Value%20Structure))
  (:Released
    (Rendering|Material|SetMaterial (Variables|Debug|GetStaticMeshComponent) 0 (.OutItem (Utilities|Array|Random (Variables|Default|GetMeshesNature))))))

(event Input|KeyboardEvents|DebugKey2
  (params (Key :type Key%20Structure :default "None") (ActionValue :type Input%20Action%20Value%20Structure))
  (:Released
    (Rendering|Material|SetMaterial (Variables|Debug|GetStaticMeshComponent) 0 (.OutItem (Utilities|Array|Random (Variables|Default|GetMeshesGoblin))))))

(event Input|KeyboardEvents|DebugKey3
  (params (Key :type Key%20Structure :default "None") (ActionValue :type Input%20Action%20Value%20Structure))
  (:Released
    (Rendering|Material|SetMaterial (Variables|Debug|GetStaticMeshComponent) 0 (.OutItem (Utilities|Array|Random (Variables|Default|GetMeshesMess))))))

(event Input|KeyboardEvents|DebugKey4
  (params (Key :type Key%20Structure :default "None") (ActionValue :type Input%20Action%20Value%20Structure))
  (:Released
    (Rendering|Material|SetMaterial (Variables|Debug|GetStaticMeshComponent) 0 (.OutItem (Utilities|Array|Random (Variables|Default|GetMeshesSewers))))))

(event Input|KeyboardEvents|DebugKey5
  (params (Key :type Key%20Structure :default "None") (ActionValue :type Input%20Action%20Value%20Structure))
  (:Released
    (Rendering|Material|SetMaterial (Variables|Debug|GetStaticMeshComponent) 0 (.OutItem (Utilities|Array|Random (Variables|Default|GetMeshesWood))))))

(event Input|KeyboardEvents|DebugKey6
  (params (Key :type Key%20Structure :default "None") (ActionValue :type Input%20Action%20Value%20Structure))
  (:Released
    (Rendering|Material|SetMaterial (Variables|Debug|GetStaticMeshComponent) 0 (.OutItem (Utilities|Array|Random (Variables|Default|GetMeshesPersian))))))

(event Input|KeyboardEvents|DebugKey7
  (params (Key :type Key%20Structure :default "None") (ActionValue :type Input%20Action%20Value%20Structure))
  (:Released
    (Rendering|Material|SetMaterial (Variables|Debug|GetStaticMeshComponent) 0 (.OutItem (Utilities|Array|Random (Variables|Default|GetMeshDefault))))))

(fn ConstructionScript)