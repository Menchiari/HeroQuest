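; BP_TriggerRoom is a room actor whose roof can be clicked to toggle its visibility along with a point light.
; On BeginPlay it shows the roof, hides the light, and randomizes light temperature plus spring arm height, yaw and length within MaxRadius.
; Roof clicks play a door sound unless the room is a Corridor.
; Releasing P toggles roof and light on every actor of this class.
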(event OnClicked(Roof)
  (params (TouchedComponent :type Primitive%20Component%20Object%20Reference) (ButtonPressed :type Key%20Structure :default "None"))
  (bind _roof (Variables|Default|GetRoof))
  (bind _pointlight (Variables|Default|GetPointLight))
  (Development|SetHiddeninGame _roof (not (Variables|/Script/Engine.SceneComponent|GetbHiddenInGame _roof)) false)
  (Development|SetHiddeninGame _pointlight (not (Variables|/Script/Engine.SceneComponent|GetbHiddenInGame _pointlight)) false)
  (if (not (Variables|Default|GetCorridor?))
    (Audio|PlaySound2D (Variables|Default|GetDoorSFX) 1.0 1.0 0.0 0 0)))

(event EventBeginPlay
  (bind _springarm (Variables|Default|GetSpringArm))
  (bind _pointlight (Variables|Default|GetPointLight))
  (bind _returnvalue (Transformation|GetWorldLocation _springarm))
  (bind _probesize (Variables|/Script/Engine.SpringArmComponent|GetProbeSize _springarm))
  (Utilities|FlowControl|Sequence
    (:then_0
      (Development|SetHiddeninGame _pointlight true false)
      (Class|LightComponent|SetTemperature _pointlight (Math|Random|RandomFloatinRange 2.5e+03 7e+03))
      (Development|SetHiddeninGame (Variables|Default|GetRoof) false false))
    (:then_1
      (Transformation|SetWorldLocation _springarm (Math|Vector|MakeVector (.x _returnvalue) (.y _returnvalue) (+ (.z _returnvalue) (Math|Random|RandomFloatinRange _probesize (- 5e+01 _probesize)))) false false)
      (Transformation|SetWorldRotation _springarm (Math|Rotator|MakeRotator 0.0 0.0 (Math|Random|RandomFloatinRange 0.0 3.6e+02)) false false)
      (Variables|/Script/Engine.SpringArmComponent|SetTargetArmLength _springarm (Math|Random|RandomFloatinRange 0.0 (Variables|Default|GetMaxRadius))))))

(event Input|KeyboardEvents|P
  (params (Key :type Key%20Structure :default "None"))
  (:Released
    (bind _outactors (Actor|GetAllActorsOfClass (Utilities|GetClass self)))
    (for _array_element _outactors
      (Development|SetHiddeninGame (Variables|BP_TriggerRoom_C|GetRoof _array_element) (not (Variables|/Script/Engine.SceneComponent|GetbHiddenInGame (Variables|BP_TriggerRoom_C|GetRoof _array_element))) false)
      (Development|SetHiddeninGame (Variables|BP_TriggerRoom_C|GetPointLight _array_element) (not (Variables|/Script/Engine.SceneComponent|GetbHiddenInGame (Variables|BP_TriggerRoom_C|GetPointLight _array_element))) false))))

(fn ConstructionScript)