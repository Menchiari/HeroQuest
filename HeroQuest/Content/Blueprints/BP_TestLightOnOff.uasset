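; BP_TestLightOnOff is a test actor that toggles a point light on and off.
; On begin play the light is hidden and the Plane is visible.
; Either the ToggleRoom event or a click on the Plane flips the hidden-in-game state of both components, keeping them opposite, and prints a debug string.
; The Trigger component's click event is left empty.
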(event OnClicked(Trigger)
  (params (TouchedComponent :type Primitive%20Component%20Object%20Reference) (ButtonPressed :type Key%20Structure :default "None")))

(event OnClicked(Plane)
  (params (TouchedComponent :type Primitive%20Component%20Object%20Reference) (ButtonPressed :type Key%20Structure :default "None"))
  (bind _plane (Variables|Default|GetPlane))
  (bind _pointlightcomponent (Variables|Default|GetPointLightComponent))
  (Development|SetHiddeninGame _plane (not (Variables|/Script/Engine.SceneComponent|GetbHiddenInGame _plane)) false)
  (Development|SetHiddeninGame _pointlightcomponent (not (Variables|/Script/Engine.SceneComponent|GetbHiddenInGame _pointlightcomponent)) false)
  (Development|PrintString "Hello"))

(event Custom|ToggleRoom
  (bind _plane (Variables|Default|GetPlane))
  (bind _pointlightcomponent (Variables|Default|GetPointLightComponent))
  (Development|SetHiddeninGame _plane (not (Variables|/Script/Engine.SceneComponent|GetbHiddenInGame _plane)) false)
  (Development|SetHiddeninGame _pointlightcomponent (not (Variables|/Script/Engine.SceneComponent|GetbHiddenInGame _pointlightcomponent)) false)
  (Development|PrintString "Hello"))

(event EventBeginPlay
  (Development|SetHiddeninGame (Variables|Default|GetPointLightComponent) true false)
  (Development|SetHiddeninGame (Variables|Default|GetPlane) false false))

(fn ConstructionScript)